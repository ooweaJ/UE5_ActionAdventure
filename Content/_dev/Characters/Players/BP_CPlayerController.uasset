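; Player controller Blueprint that handles input for toggling the inventory and store screens on the main player UI.
; IA_Tab and IA_F Enhanced Input actions each cast MainWidget to UI_PlayerMain and call ShowInventory or ShowStore respectively.
; Each action has its own FlipFlop alternating show and hide, so it tracks toggle state independently of the widget's actual visibility.
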(event Input|EnhancedActionEvents|EnhancedInputActionIA_Tab
  (params (ActionValue :type Boolean) (ElapsedSeconds :type Float%20%28double-precision%29) (TriggeredSeconds :type Float%20%28double-precision%29) (InputAction :type Input%20Action%20Object%20Reference :default "/Game/_dev/Characters/Players/Input/IA_Tab.IA_Tab"))
  (:Started
    (bind _asui_player_main (Utilities|Casting|CastToUI_PlayerMain (Variables|Default|GetMainWidget)))
    (Utilities|FlowControl|FlipFlop
      (:A
        (Default|ShowInventory _asui_player_main true))
      (:B
        (Default|ShowInventory _asui_player_main false)))))

(event Input|EnhancedActionEvents|EnhancedInputActionIA_F
  (params (ActionValue :type Boolean) (ElapsedSeconds :type Float%20%28double-precision%29) (TriggeredSeconds :type Float%20%28double-precision%29) (InputAction :type Input%20Action%20Object%20Reference :default "/Game/_dev/Characters/Players/Input/IA_F.IA_F"))
  (:Started
    (bind _asui_player_main (Utilities|Casting|CastToUI_PlayerMain (Variables|Default|GetMainWidget)))
    (Utilities|FlowControl|FlipFlop
      (:A
        (Default|ShowStore _asui_player_main true))
      (:B
        (Default|ShowStore _asui_player_main false)))))

(event EventBeginPlay)

(event EventTick
  (params (DeltaSeconds :type Float%20%28single-precision%29)))

(fn ConstructionScript)