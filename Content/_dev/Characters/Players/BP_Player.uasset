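; BP_Player is a player character Blueprint with a keyboard toggle between two body meshes.
; Pressing M flip-flops between assigning UE4_Mannequin to the SkeletalMesh component while hiding Mesh, and clearing that asset while showing Mesh again.
; An unconnected debug chain compares the stored capsule forward vector with the current right vector by dot product to print F, R or L for turn direction.
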(event EventBeginPlay)

(event EventTick
  (params (DeltaSeconds :type Float%20%28single-precision%29)))

(event Input|KeyboardEvents|M
  (params (Key :type Key%20Structure :default "None"))
  (bind _skeletalmesh (Variables|Default|GetSkeletalMesh))
  (bind _mesh (Variables|Character|GetMesh))
  (:Pressed
    (Utilities|FlowControl|FlipFlop
      (:A
        (Components|SkinnedMesh|SetSkinnedAssetandUpdate _skeletalmesh "/Game/Scanned3DPeoplePack/RP_Character/00_rp_master/Mannequin/UE4_Mannequin.UE4_Mannequin" true)
        (Rendering|SetVisibility _mesh false false))
      (:B
        (Components|SkinnedMesh|SetSkinnedAssetandUpdate _skeletalmesh 0 true)
        (Rendering|SetVisibility _mesh true false)))))

(event Input|KeyboardEvents|Q
  (params (Key :type Key%20Structure :default "None")))

(fn ConstructionScript)