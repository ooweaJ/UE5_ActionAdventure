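; BP_AttackCircle is a timed attack telegraph actor that shows a circle, fills its area, then triggers an attack.
; On BeginPlay, it creates dynamic materials for the Circum and Area components, using the Circum1Area0 parameter to distinguish outline from fill.
; After a short delay, a timeline animates the area material's AreaValue.
; When the timeline finishes, it calls SpawnAttack and destroys itself shortly afterward.
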(event EventBeginPlay
  (Utilities|FlowControl|Sequence
    (:then_0
      (bind _returnvalue (Rendering|Material|CreateDynamicMaterialInstance (Variables|Default|GetCircum) :!class /Script/Engine.DecalComponent))
      (bind _output_get (Variables|Default|SetCirumRef _returnvalue))
      (Rendering|Material|SetScalarParameterValue _output_get "Circum1Area0" 1.0 :!class /Script/Engine.MaterialInstanceDynamic))
    (:then_1
      (bind _returnvalue_2 (Rendering|Material|CreateDynamicMaterialInstance (Variables|Default|GetArea) :!class /Script/Engine.DecalComponent))
      (bind _output_get_2 (Variables|Default|SetAreaRef _returnvalue_2))
      (Rendering|Material|SetScalarParameterValue _output_get_2 "Circum1Area0" 0.0 :!class /Script/Engine.MaterialInstanceDynamic))
    (:then_2
      (Utilities|FlowControl|Delay 0.5)
      (bind _새_트랙_0 (Timeline|타임라인 Play)
        (:Update
          (Rendering|Material|SetScalarParameterValue (Variables|Default|GetAreaRef) "AreaValue" _새_트랙_0 :!class /Script/Engine.MaterialInstanceDynamic))
        (:Finished
          (Class|BossRange|SpawnAttack)
          (Utilities|FlowControl|Delay 0.2)
          (Actor|DestroyActor))))))

(event Collision|EventActorBeginOverlap
  (params (OtherActor :type Actor%20Object%20Reference)))

(event EventTick
  (params (DeltaSeconds :type Float%20%28single-precision%29)))

(fn ConstructionScript)